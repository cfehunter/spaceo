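; HUD Blueprint that draws a simple minimap of Room actors and MyCharacter actors, anchored at the horizontal center near the top of the screen.
; Each DrawHUD call finds all actors of both classes, scales their XY world positions down and rotates them 45 degrees around Z.
; Rooms appear as small rotated brick-textured squares, with characters drawn afterward as larger icons.
; Positions are relative to the world origin, so the map does not follow the player.
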(event EventDrawHUD
  (params (SizeX :type Integer) (SizeY :type Integer))
  (Variables|Default|SetScreenMidX (/ (Math|Conversions|ToFloat(Integer) SizeX) 2.0))
  (Variables|Default|SetScreenMidY (/ (Math|Conversions|ToFloat(Integer) SizeY) 2e+01))
  (bind _outactors (Actor|GetAllActorsOfClass "/Script/ggj_2015.Room"))
  (for _array_element _outactors
    (bind _asroom (Utilities|Casting|CastToRoom _array_element))
    (Canvas|DrawTexture "/Game/StarterContent/Textures/T_Brick_Clay_New_D.T_Brick_Clay_New_D" (+ (.X (Math|Vector|BreakVector (Math|Vector|RotateVectorAroundAxis (Math|Vector|MakeVector (/ (.X (Math|Vector|BreakVector (Transformation|GetActorLocation _asroom))) 4e+01) (/ (.Y (Math|Vector|BreakVector (Transformation|GetActorLocation _asroom))) 4e+01) 0.0) 45.0 "0,0.000000,1.000000"))) (Variables|Default|GetScreenMidX)) (+ (.Y (Math|Vector|BreakVector (Math|Vector|RotateVectorAroundAxis (Math|Vector|MakeVector (/ (.X (Math|Vector|BreakVector (Transformation|GetActorLocation _asroom))) 4e+01) (/ (.Y (Math|Vector|BreakVector (Transformation|GetActorLocation _asroom))) 4e+01) 0.0) 45.0 "0,0.000000,1.000000"))) (Variables|Default|GetScreenMidY)) 8.0 8.0 0.0 0.0 1.0 1.0 "(R=1.000000,G=1.000000,B=1.000000,A=1.000000)" "BLEND_Translucent" 1.0 false 45.0))
  (bind _outactors_2 (Actor|GetAllActorsOfClass "/Game/Blueprints/MyCharacter.MyCharacter_C"))
  (for _array_element_2 _outactors_2
    (bind _asmy_character (Utilities|Casting|CastToMyCharacter _array_element_2))
    (Canvas|DrawTexture "/Game/Environment/ImportantIcon.ImportantIcon" (+ (.X (Math|Vector|BreakVector (Math|Vector|RotateVectorAroundAxis (Math|Vector|MakeVector (/ (.X (Math|Vector|BreakVector (Transformation|GetActorLocation _asmy_character))) 4e+01) (/ (.Y (Math|Vector|BreakVector (Transformation|GetActorLocation _asmy_character))) 4e+01) 0.0) 45.0 "0,0.000000,1.000000"))) (Variables|Default|GetScreenMidX)) (+ (.Y (Math|Vector|BreakVector (Math|Vector|RotateVectorAroundAxis (Math|Vector|MakeVector (/ (.X (Math|Vector|BreakVector (Transformation|GetActorLocation _asmy_character))) 4e+01) (/ (.Y (Math|Vector|BreakVector (Transformation|GetActorLocation _asmy_character))) 4e+01) 0.0) 45.0 "0,0.000000,1.000000"))) (Variables|Default|GetScreenMidY)) 16.0 16.0 1.0 1.0 1.0 1.0 "(R=1.000000,G=1.000000,B=1.000000,A=1.000000)" "BLEND_Translucent" 1.0 false 0.0)))

(fn ConstructionScript)