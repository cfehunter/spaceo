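; Player character Blueprint that handles an objective pickup, its turn-in and damage from beasts.
; A capsule overlap with a matching actor class destroys that actor, sets a powerup flag and plays a voice cue.
; Hitting a matching class while flagged plays mission complete and clears the flag.
; Otherwise, hitting a Beast_Character subtracts its Attack from Health, hiding the player and disabling input below 1.
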(event OnComponentBeginOverlap(CapsuleComponent)
  (params (OtherActor :type Actor%20Object%20Reference) (OtherComp :type Primitive%20Component%20Object%20Reference) (OtherBodyIndex :type Integer) (bFromSweep :type Boolean) (SweepResult :type Hit%20Result%20Structure%20%28by%20ref%29))
  (if (Utilities|ClassIsChildOf (Utilities|GetClass OtherActor) 0)
    (Actor|DestroyActor OtherActor)
    (Variables|Default|SetHasObjectivePowerup true)
    (Audio|PlaySoundatLocation "/Game/SFX/EngiGoodWork.EngiGoodWork" "0, 0, 0")))

(event EventHit
  (params (MyComp :type Primitive%20Component%20Object%20Reference) (Other :type Actor%20Object%20Reference) (OtherComp :type Primitive%20Component%20Object%20Reference) (bSelfMoved :type Boolean) (HitLocation :type Vector :default "0, 0, 0") (HitNormal :type Vector :default "0, 0, 0") (NormalImpulse :type Vector :default "0, 0, 0") (Hit :type Hit%20Result%20Structure%20%28by%20ref%29))
  (bind _returnvalue (Utilities|GetClass Other))
  (if (Utilities|ClassIsChildOf _returnvalue 0)
    (if (Variables|Default|GetHasObjectivePowerup)
      (Audio|PlaySoundatLocation "/Game/SFX/EngiMissionComplete.EngiMissionComplete" "0, 0, 0")
      (Variables|Default|SetHasObjectivePowerup false))
    (elif (== _returnvalue "/Game/AI/Beast_Character.Beast_Character_C")
      (bind _asbeast_character (Utilities|Casting|CastToBeast_Character Other))
      (Variables|Default|SetHealth (- (Variables|Default|GetHealth) (Variables|/Game/AI/Beast_Character.Beast_Character_C|GetAttack _asbeast_character)))
      (if (< (Variables|Default|GetHealth) 1)
        (Rendering|SetActorHiddenInGame true)
        (Input|DisableInput 0)))))

(fn ConstructionScript)